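; Vehicle movement component that drives its owning actor kinematically, exposing Accelerate, StopAcclerating and Turn events plus speed and velocity getters.
; Accelerate interpolates speed toward forward or reverse limits, while Tick eases it to zero when not accelerating and prints it for debugging.
; Both move the owner along its forward vector by unswept per-call offsets, not scaled by delta time.
; Turn applies smoothed yaw that depends on current speed and its sign.
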(event `self.ReceiveTick`
  (params (DeltaSeconds :type "Float (single-precision)"))
  (bind _returnvalue (`KismetMathLibrary.FInterpTo` (`self.CurrentSpeed`) 0.0 (`GameplayStatics.GetWorldDeltaSeconds`) (`self.Deceleration`)))
  (`|ExecutionSequence`
    (:`then_0`
      (if (not (`self.IsAccelerating`))
        (`|ExecutionSequence`
          (:`then_0`
            (set `self.CurrentSpeed` _returnvalue))
          (:`then_1`
            (set `self.Velocity` (* (`Actor.GetActorForwardVector` (`self.GetOwner`)) _returnvalue)))
          (:`then_2`
            (`Actor.K2_AddActorWorldOffset` (`self.GetOwner`) (`self.Velocity`) false false)))))
    (:`then_1`
      (`KismetSystemLibrary.PrintString` (`KismetStringLibrary.Conv_DoubleToString` (`self.CurrentSpeed`)) true true (struct :`G` 0.66 :`B` 1.0 :`A` 1.0) 0.0))))

(event `Accelerate`
  (params (InputValue :type "Float (double-precision)"))
  (bind _returnvalue (`KismetMathLibrary.FInterpTo` (`self.CurrentSpeed`) (* (`KismetMathLibrary.SelectFloat` (`self.MaxSpeed`) (`self.MaxSpeedBackward`) (> InputValue 0.0)) InputValue) (`GameplayStatics.GetWorldDeltaSeconds`) (`self.Acceleration`)))
  (set `self.IsAccelerating` true)
  (`|ExecutionSequence`
    (:`then_0`
      (set `self.CurrentSpeed` _returnvalue))
    (:`then_1`
      (set `self.Velocity` (`Actor.GetActorForwardVector` (`self.GetOwner`))))
    (:`then_2`
      (`Actor.K2_AddActorWorldOffset` (`self.GetOwner`) (* (`self.Velocity`) _returnvalue) false false))))

(event `StopAcclerating`
  (set `self.IsAccelerating` false))

(event `Turn`
  (params (InputValue :type "Float (double-precision)"))
  (set `self.TurnFactor` (`KismetMathLibrary.FInterpTo` (`self.TurnFactor`) (* (* (* (`self.MaxTurnSpeed`) InputValue (`KismetMathLibrary.Lerp` 2.5 1.0 (/ (`KismetMathLibrary.Abs` (`self.CurrentSpeed`)) (`self.Acceleration`)))) (`GameplayStatics.GetWorldDeltaSeconds`)) (/ (`self.CurrentSpeed`) (`self.MaxSpeed`))) (`GameplayStatics.GetWorldDeltaSeconds`) (`self.TurnInterpolationSpeed`)))
  (`Actor.K2_AddActorWorldRotation` (`self.GetOwner`) (`KismetMathLibrary.MakeRotator` 0.0 0.0 (`self.TurnFactor`)) false false))

(fn `GetCurrentSpeed`
  (returns (ReturnValue :type "Float (double-precision)"))
  (return (`self.CurrentSpeed`)))

(fn `GetVelocity`
  (returns (Velocity :type "Vector Structure"))
  (return (`self.Velocity`)))