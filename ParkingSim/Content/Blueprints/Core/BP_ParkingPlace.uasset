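; Parking spot actor that detects when a vehicle is fully parked inside its trigger Box.
; Overlapping BoxComponents are tracked without duplicates, and the vehicle counts as parked while at least four are inside.
; Each new overlap starts a three-second Delay, ignored if already running, then prints a win message if still parked.
; Debug prints show tracked component names every tick and the parked state on exit.
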(event `self.ReceiveTick`
  (params (DeltaSeconds :type "Float (single-precision)"))
  (for _array_element (`self.BoxDetection`)
    (`KismetSystemLibrary.PrintString` (`KismetSystemLibrary.GetDisplayName` _array_element) true true (struct :`G` 0.66 :`B` 1.0 :`A` 1.0) 0.0)))

(event `self.Box.OnComponentBeginOverlap`
  (params (OverlappedComponent :type "PrimitiveComponent Object Reference") (OtherActor :type "Actor Object Reference") (OtherComp :type "PrimitiveComponent Object Reference") (OtherBodyIndex :type Integer) (bFromSweep :type Boolean) (SweepResult :type "HitResult Structure (by ref)"))
  (bind _boxdetection (`self.BoxDetection`))
  (if (and (== (`GameplayStatics.GetObjectClass` OtherComp) "/Script/Engine.BoxComponent") (== (`KismetArrayLibrary.Array_Find` (`self.BoxDetection`) OtherComp) -1))
    (`KismetArrayLibrary.Array_Add` _boxdetection OtherComp)
    (set `self.IsVehiculeParked` (>= (`KismetArrayLibrary.Array_Length` _boxdetection) 4))
    (`KismetSystemLibrary.Delay` 3.0)
    (if (`self.IsVehiculeParked`)
      (`KismetSystemLibrary.PrintString` "Win !"))))

(event `self.Box.OnComponentEndOverlap`
  (params (OverlappedComponent :type "PrimitiveComponent Object Reference") (OtherActor :type "Actor Object Reference") (OtherComp :type "PrimitiveComponent Object Reference") (OtherBodyIndex :type Integer))
  (bind _boxdetection (`self.BoxDetection`))
  (`KismetArrayLibrary.Array_RemoveItem` _boxdetection OtherComp)
  (bind _output_get (set `self.IsVehiculeParked` (>= (`KismetArrayLibrary.Array_Length` _boxdetection) 4)))
  (`KismetSystemLibrary.PrintString` (`KismetStringLibrary.Conv_BoolToString` _output_get)))

(fn `UserConstructionScript`)